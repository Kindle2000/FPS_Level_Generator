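; M4A1 weapon Blueprint that handles firing and reloading for the player's rifle.
; Shoot spawns a BP_BaseBullet at the muzzle socket, decrements Ammo without checking it, and spawns a scaled-down muzzle flash on player 0's equipped weapon.
; Reload tops up the clip from the MaxAmmo reserve, or takes what remains, then sets IsReloading on the ThirdPersonCharacter.
; A full clip only prints a message.
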(event Custom|Shoot
  (Game|SpawnActorfromClass "/Game/ThirdPersonBP/Blueprints/BP_BaseBullet.BP_BaseBullet_C" (Transformation|GetSocketTransform (Variables|Default|GetSkeletalMesh) "Muzzel" "RTS_World") "Undefined" 0 0)
  (Variables|Default|SetAmmo (- (Variables|Default|GetAmmo) 1))
  (bind _asthird_person_character (Utilities|Casting|CastToThirdPersonCharacter (Game|GetPlayerCharacter 0)))
  (bind _returnvalue (Effects|SpawnEmitteratLocation "/Game/InfinityBladeEffects/Effects/FX_Monsters/FX_Monster_Chicken/P_ChickenMaster_MuzzleFlash_01.P_ChickenMaster_MuzzleFlash_01" (Transformation|GetSocketLocation (Variables|/Game/ShooterContent/FPSAssets/Weapon/AK-47/BP_WeaponBase.BP_WeaponBase_C|GetSkeletalMesh (Variables|/Game/ThirdPersonBP/Blueprints/ThirdPersonCharacter.ThirdPersonCharacter_C|GetEquippedWeapon _asthird_person_character)) "Muzzel") (Transformation|GetSocketRotation (Variables|/Game/ShooterContent/FPSAssets/Weapon/AK-47/BP_WeaponBase.BP_WeaponBase_C|GetSkeletalMesh (Variables|/Game/ThirdPersonBP/Blueprints/ThirdPersonCharacter.ThirdPersonCharacter_C|GetEquippedWeapon _asthird_person_character)) "Muzzel")))
  (Transformation|SetWorldScale3D _returnvalue "0.050000,0.050000,0.050000"))

(event EventBeginPlay)

(event Collision|EventActorBeginOverlap
  (params (OtherActor :type Actor%20Object%20Reference)))

(event EventTick
  (params (DeltaSeconds :type Float%20%28single-precision%29)))

(fn ConstructionScript)

(fn Reload
  (if (< (Variables|Default|GetAmmo) (Variables|Default|GetClipSize))
    (if (> (Variables|Default|GetMaxAmmo) (- (Variables|Default|GetClipSize) (Variables|Default|GetAmmo)))
      (Variables|Default|SetAmmoDiff (- (Variables|Default|GetClipSize) (Variables|Default|GetAmmo)))
      (Variables|Default|SetAmmo (+ (Variables|Default|GetAmmoDiff) (Variables|Default|GetAmmo)))
      (Variables|Default|SetMaxAmmo (- (Variables|Default|GetMaxAmmo) (Variables|Default|GetAmmoDiff)))
      (bind _asthird_person_character (Utilities|Casting|CastToThirdPersonCharacter (Game|GetPlayerCharacter 0)))
      (bind _output_get (Variables|/Game/ThirdPersonBP/Blueprints/ThirdPersonCharacter.ThirdPersonCharacter_C|SetIsReloading _asthird_person_character true))
      (return (stale _output_get_2) _output_get)
      (else
        (Variables|Default|SetAmmoDiff (- (Variables|Default|GetClipSize) (Variables|Default|GetAmmo)))
        (Variables|Default|SetAmmo (+ (Variables|Default|GetAmmo) (Variables|Default|GetMaxAmmo)))
        (Variables|Default|SetMaxAmmo 0)
        (bind _asthird_person_character_2 (Utilities|Casting|CastToThirdPersonCharacter (Game|GetPlayerCharacter 0)))
        (bind _output_get_2 (Variables|/Game/ThirdPersonBP/Blueprints/ThirdPersonCharacter.ThirdPersonCharacter_C|SetIsReloading _asthird_person_character_2 true))))
    (else
      (Development|PrintString "Full Ammo"))))