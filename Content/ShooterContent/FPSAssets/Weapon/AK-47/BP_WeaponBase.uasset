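; Base weapon Blueprint that handles hitscan shooting and reloading for the player's ThirdPersonCharacter.
; Shoot plays audio, traces from the ADS or follow camera depending on aiming, spends ammo and spawns a muzzle flash.
; Hits on CBP_SimpleEnemy show a hit marker and subtract health, then either spawn an impact effect or trigger ragdoll and kill feed.
; Reload refills Ammo from MaxAmmo and flags the character as reloading; projectile spawning is unconnected.
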(event Custom|Shoot
  (Audio|Components|Audio|Play (Variables|Default|GetAudio) 0.0)
  (bind _asthird_person_character (Utilities|Casting|CastToThirdPersonCharacter (Game|GetPlayerCharacter 0)))
  (if (Variables|/Game/ThirdPersonBP/Blueprints/ThirdPersonCharacter.ThirdPersonCharacter_C|GetIsAiming _asthird_person_character)
    (bind _outhit (Collision|LineTraceByChannel (Transformation|GetWorldLocation (Variables|/Game/ThirdPersonBP/Blueprints/ThirdPersonCharacter.ThirdPersonCharacter_C|GetADSCam _asthird_person_character)) (+ (Transformation|GetWorldLocation (Variables|/Game/ThirdPersonBP/Blueprints/ThirdPersonCharacter.ThirdPersonCharacter_C|GetADSCam _asthird_person_character)) (* (Math|Vector|GetForwardVector (Transformation|GetWorldRotation (Variables|/Game/ThirdPersonBP/Blueprints/ThirdPersonCharacter.ThirdPersonCharacter_C|GetADSCam _asthird_person_character))) 1.5e+03)) "TraceTypeQuery1" false 0 "None"))
    (Variables|Default|SetAmmo (- (Variables|Default|GetAmmo) 1))
    (bind _asthird_person_character_2 (Utilities|Casting|CastToThirdPersonCharacter (Game|GetPlayerCharacter 0)))
    (bind _returnvalue (Effects|SpawnEmitteratLocation "/Game/InfinityBladeEffects/Effects/FX_Monsters/FX_Monster_Chicken/P_ChickenMaster_MuzzleFlash_01.P_ChickenMaster_MuzzleFlash_01" (Transformation|GetSocketLocation (Variables|BP_WeaponBase_C|GetSkeletalMesh (Variables|/Game/ThirdPersonBP/Blueprints/ThirdPersonCharacter.ThirdPersonCharacter_C|GetEquippedWeapon _asthird_person_character_2)) "Muzzel") (Transformation|GetSocketRotation (Variables|BP_WeaponBase_C|GetSkeletalMesh (Variables|/Game/ThirdPersonBP/Blueprints/ThirdPersonCharacter.ThirdPersonCharacter_C|GetEquippedWeapon _asthird_person_character_2)) "Muzzel")))
    (Transformation|SetWorldScale3D _returnvalue "0.050000,0.050000,0.050000")
    (bind _ascbp_simple_enemy (Utilities|Casting|CastToCBP_SimpleEnemy (.HitActor (Collision|BreakHitResult _outhit))))
    (bind _returnvalue_2 (UserInterface|CreateWidget "/Game/ShooterContent/FPSAssets/WBP_HitMarker.WBP_HitMarker_C"))
    (UserInterface|Viewport|AddtoViewport _returnvalue_2 0)
    (bind _output_get (Variables|/Game/ThirdPersonBP/Blueprints/CBP_SimpleEnemy.CBP_SimpleEnemy_C|SetHealth _ascbp_simple_enemy (- (Variables|/Game/ThirdPersonBP/Blueprints/CBP_SimpleEnemy.CBP_SimpleEnemy_C|GetHealth _ascbp_simple_enemy) (Variables|Default|GetDamge))))
    (if (<= _output_get 0.0)
      (if (not (Variables|/Game/ThirdPersonBP/Blueprints/CBP_SimpleEnemy.CBP_SimpleEnemy_C|GetDead _ascbp_simple_enemy))
        (Physics|SetSimulatePhysics (Variables|/Script/Engine.Character|GetMesh _ascbp_simple_enemy) true)
        (bind _returnvalue_3 (UserInterface|CreateWidget "/Game/ThirdPersonBP/Blueprints/WBP_KillFeed.WBP_KillFeed_C"))
        (UserInterface|Viewport|AddtoViewport _returnvalue_3 0)
        (Variables|/Game/ThirdPersonBP/Blueprints/CBP_SimpleEnemy.CBP_SimpleEnemy_C|SetDead _ascbp_simple_enemy true))
      (else
        (Effects|SpawnEmitteratLocation "/Game/InfinityBladeEffects/Effects/FX_Mobile/ICE/combat/P_Impact_Shield.P_Impact_Shield" (.Location (Collision|BreakHitResult _outhit)))))
    (else
      (bind _outhit_2 (Collision|LineTraceByChannel (Transformation|GetWorldLocation (Variables|/Game/ThirdPersonBP/Blueprints/ThirdPersonCharacter.ThirdPersonCharacter_C|GetFollowCamera _asthird_person_character)) (+ (Transformation|GetWorldLocation (Variables|/Game/ThirdPersonBP/Blueprints/ThirdPersonCharacter.ThirdPersonCharacter_C|GetFollowCamera _asthird_person_character)) (* (Math|Vector|GetForwardVector (Transformation|GetWorldRotation (Variables|/Game/ThirdPersonBP/Blueprints/ThirdPersonCharacter.ThirdPersonCharacter_C|GetFollowCamera _asthird_person_character))) 1.5e+03)) "TraceTypeQuery1" false 0 "None"))
      (Variables|Default|SetAmmo (- (Variables|Default|GetAmmo) 1))
      (bind _asthird_person_character_3 (Utilities|Casting|CastToThirdPersonCharacter (Game|GetPlayerCharacter 0)))
      (bind _returnvalue_4 (Effects|SpawnEmitteratLocation "/Game/InfinityBladeEffects/Effects/FX_Monsters/FX_Monster_Chicken/P_ChickenMaster_MuzzleFlash_01.P_ChickenMaster_MuzzleFlash_01" (Transformation|GetSocketLocation (Variables|BP_WeaponBase_C|GetSkeletalMesh (Variables|/Game/ThirdPersonBP/Blueprints/ThirdPersonCharacter.ThirdPersonCharacter_C|GetEquippedWeapon _asthird_person_character_3)) "Muzzel") (Transformation|GetSocketRotation (Variables|BP_WeaponBase_C|GetSkeletalMesh (Variables|/Game/ThirdPersonBP/Blueprints/ThirdPersonCharacter.ThirdPersonCharacter_C|GetEquippedWeapon _asthird_person_character_3)) "Muzzel")))
      (Transformation|SetWorldScale3D _returnvalue_4 "0.050000,0.050000,0.050000")
      (bind _ascbp_simple_enemy_2 (Utilities|Casting|CastToCBP_SimpleEnemy (.HitActor (Collision|BreakHitResult _outhit_2))))
      (bind _returnvalue_5 (UserInterface|CreateWidget "/Game/ShooterContent/FPSAssets/WBP_HitMarker.WBP_HitMarker_C"))
      (UserInterface|Viewport|AddtoViewport _returnvalue_5 0)
      (bind _output_get_2 (Variables|/Game/ThirdPersonBP/Blueprints/CBP_SimpleEnemy.CBP_SimpleEnemy_C|SetHealth _ascbp_simple_enemy_2 (- (Variables|/Game/ThirdPersonBP/Blueprints/CBP_SimpleEnemy.CBP_SimpleEnemy_C|GetHealth _ascbp_simple_enemy_2) (Variables|Default|GetDamge))))
      (if (<= _output_get_2 0.0)
        (if (not (Variables|/Game/ThirdPersonBP/Blueprints/CBP_SimpleEnemy.CBP_SimpleEnemy_C|GetDead _ascbp_simple_enemy_2))
          (Physics|SetSimulatePhysics (Variables|/Script/Engine.Character|GetMesh _ascbp_simple_enemy_2) true)
          (bind _returnvalue_6 (UserInterface|CreateWidget "/Game/ThirdPersonBP/Blueprints/WBP_KillFeed.WBP_KillFeed_C"))
          (UserInterface|Viewport|AddtoViewport _returnvalue_6 0)
          (Variables|/Game/ThirdPersonBP/Blueprints/CBP_SimpleEnemy.CBP_SimpleEnemy_C|SetDead _ascbp_simple_enemy_2 true))
        (else
          (Effects|SpawnEmitteratLocation "/Game/InfinityBladeEffects/Effects/FX_Mobile/ICE/combat/P_Impact_Shield.P_Impact_Shield" (.Location (Collision|BreakHitResult _outhit_2))))))))

(event EventBeginPlay)

(event Collision|EventActorBeginOverlap
  (params (OtherActor :type Actor%20Object%20Reference)))

(event EventTick
  (params (DeltaSeconds :type Float%20%28single-precision%29)))

(fn ConstructionScript)

(fn Reload
  (if (< (Variables|Default|GetAmmo) (Variables|Default|GetClipSize))
    (if (> (Variables|Default|GetMaxAmmo) (- (Variables|Default|GetClipSize) (Variables|Default|GetAmmo)))
      (Variables|Default|SetAmmoDiff (- (Variables|Default|GetClipSize) (Variables|Default|GetAmmo)))
      (Variables|Default|SetAmmo (+ (Variables|Default|GetAmmoDiff) (Variables|Default|GetAmmo)))
      (Variables|Default|SetMaxAmmo (- (Variables|Default|GetMaxAmmo) (Variables|Default|GetAmmoDiff)))
      (bind _asthird_person_character (Utilities|Casting|CastToThirdPersonCharacter (Game|GetPlayerCharacter 0)))
      (bind _output_get (Variables|/Game/ThirdPersonBP/Blueprints/ThirdPersonCharacter.ThirdPersonCharacter_C|SetIsReloading _asthird_person_character true))
      (return _output_get)
      (else
        (Variables|Default|SetAmmoDiff (- (Variables|Default|GetClipSize) (Variables|Default|GetAmmo)))
        (Variables|Default|SetAmmo (+ (Variables|Default|GetAmmo) (Variables|Default|GetMaxAmmo)))
        (Variables|Default|SetMaxAmmo 0)
        (bind _asthird_person_character_2 (Utilities|Casting|CastToThirdPersonCharacter (Game|GetPlayerCharacter 0)))
        (bind _output_get_2 (Variables|/Game/ThirdPersonBP/Blueprints/ThirdPersonCharacter.ThirdPersonCharacter_C|SetIsReloading _asthird_person_character_2 true))
        (return _output_get_2)))
    (else
      (Development|PrintString "Full Ammo"))))