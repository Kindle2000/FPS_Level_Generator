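; Grid generator actor that spawns a scaled, evenly spaced field of tile actors from Width, Height and Spacing.
; MakeTiles destroys and clears the previous tiles, then runs nested loops to spawn new ones offset in X/Y from the actor, passing each its grid coordinates.
; The construction script holds only leftover empty loops and does not call MakeTiles; the event graph is unused.
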(event EventBeginPlay)

(event Collision|EventActorBeginOverlap
  (params (OtherActor :type Actor%20Object%20Reference)))

(event EventTick
  (params (DeltaSeconds :type Float%20%28single-precision%29)))

(fn ConstructionScript
  (for _index (range 0 (Variables|Default|GetHeight))
    (Variables|Default|SetYIterator _index)
    (for _index_2 (range 0 (Variables|Default|GetWidth))
      _)))

(fn MakeTiles
  (bind _returnvalue (Transformation|GetActorLocation))
  (bind _scale (Variables|Default|GetScale))
  (for _array_element (Variables|Default|GetTile)
    (Utilities|IsValid _array_element
      (:Is%20Valid
        (Actor|DestroyActor _array_element))))
  (Utilities|Array|Clear (Variables|Default|GetTile))
  (for _index (range 0 (Variables|Default|GetHeight))
    (Variables|Default|SetYIterator _index)
    (for _index_2 (range 0 (Variables|Default|GetWidth))
      (bind _returnvalue_2 (Game|SpawnActorfromClass "/Game/Tile.Tile_C" (Math|Transform|MakeTransform (Math|Vector|MakeVector (+ (* _index_2 (Variables|Default|GetSpacing)) (.x _returnvalue)) (+ (.y _returnvalue) (* (Variables|Default|GetYIterator) (Variables|Default|GetSpacing))) 0.0) "0, 0, 0" (Math|Vector|MakeVector _scale _scale _scale)) "Undefined" 0 (Utilities|Struct|MakeCoord _index_2 _index) 0))
      (Utilities|Array|Add (Variables|Default|GetTile) _returnvalue_2))))